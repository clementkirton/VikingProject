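; BP_Father is a father NPC that walks toward a BP_Movepoint and plays one-time voice lines while the player pawn is nearby.
; Two overlap volumes set flags read on Tick: PlayerInRange starts or halts movement through the movement mode, and PlayerInRangeSlow selects the faster walk speed.
; SimpleMoveToActor drives the walk to the first movepoint found at BeginPlay.
; DoOnce-gated sounds fire after startup, while in range, and on nearing the goal.
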(event OnComponentBeginOverlap(PlayerinRange)
  (params (OverlappedComponent :type Primitive%20Component%20Object%20Reference) (OtherActor :type Actor%20Object%20Reference) (OtherComp :type Primitive%20Component%20Object%20Reference) (OtherBodyIndex :type Integer) (bFromSweep :type Boolean) (SweepResult :type Hit%20Result%20Structure%20%28by%20ref%29))
  ;[1 1 1] Had to add A collider to the VR pawn.
  (if (== (Game|Player|GetPlayerPawn 0) OtherActor)
    (Variables|Default|SetIs%20Player%20in%20Range true)))

(event OnComponentEndOverlap(PlayerinRange)
  (params (OverlappedComponent :type Primitive%20Component%20Object%20Reference) (OtherActor :type Actor%20Object%20Reference) (OtherComp :type Primitive%20Component%20Object%20Reference) (OtherBodyIndex :type Integer))
  ;[1 1 1] Had to add A collider to the VR pawn.
  (if (== (Game|Player|GetPlayerPawn 0) OtherActor)
    (Variables|Default|SetIs%20Player%20in%20Range false)))

(event OnComponentBeginOverlap(PlayerinRangeSlow)
  (params (OverlappedComponent :type Primitive%20Component%20Object%20Reference) (OtherActor :type Actor%20Object%20Reference) (OtherComp :type Primitive%20Component%20Object%20Reference) (OtherBodyIndex :type Integer) (bFromSweep :type Boolean) (SweepResult :type Hit%20Result%20Structure%20%28by%20ref%29))
  (if (== (Game|Player|GetPlayerPawn 0) OtherActor)
    (Variables|Default|SetIs%20Player%20in%20RangeSlow true)))

(event OnComponentEndOverlap(PlayerinRangeSlow)
  (params (OverlappedComponent :type Primitive%20Component%20Object%20Reference) (OtherActor :type Actor%20Object%20Reference) (OtherComp :type Primitive%20Component%20Object%20Reference) (OtherBodyIndex :type Integer))
  (if (== (Game|Player|GetPlayerPawn 0) OtherActor)
    (Variables|Default|SetIs%20Player%20in%20RangeSlow false)))

(event EventTick
  (params (DeltaSeconds :type Float%20%28single-precision%29))
  (bind _returnvalue (Transformation|GetActorLocation))
  (bind _returnvalue_2 (Pawn|GetController))
  (bind _charactermovement (Variables|Character|GetCharacterMovement))
  ;[1 1 1] Start/Stop Walking
  (if (Variables|Default|GetIs%20Player%20in%20Range)
    (Utilities|FlowControl|Sequence
      (:then_0
        (if (Variables|Default|GetIs%20Player%20in%20RangeSlow)
          (Pawn|Components|CharacterMovement|SetMovementMode _charactermovement "MOVE_Walking" 0)
          (Variables|/Script/Engine.CharacterMovementComponent|SetMaxWalkSpeed _charactermovement 2e+02)
          (else
            (Pawn|Components|CharacterMovement|SetMovementMode _charactermovement "MOVE_Walking" 0)
            (Variables|/Script/Engine.CharacterMovementComponent|SetMaxWalkSpeed _charactermovement 1e+02)))
        (AI|Navigation|SimpleMovetoActor _returnvalue_2 (Utilities|Array|Get(acopy) (stale EventBeginPlay _outactors)))
        (if (< (Transformation|GetDistanceTo _returnvalue_2 (Utilities|Array|Get(acopy) (stale EventBeginPlay _outactors))) 5.0)
          (Utilities|FlowControl|DoOnce false
            (:Completed
              (Audio|PlaySoundatLocation "/Game/Audio/Voice/Grab_His_Possessions_Cue.Grab_His_Possessions_Cue" (Transformation|GetActorLocation) "0, 0, 0" 1.0 1.0 0.0 0 0 0)))))
      (:then_1
        (Utilities|FlowControl|DoOnce false
          (:Completed
            (Audio|SpawnSoundatLocation "/Game/Audio/Voice/Don_t_Forget_Your_Bow_Cue.Don_t_Forget_Your_Bow_Cue" _returnvalue "0, 0, 0" 1.0 1.0 0.0 0 0))))
      (:then_2
        (Utilities|FlowControl|Delay 4.0)
        (Utilities|FlowControl|DoOnce false
          (:Completed
            (Audio|PlaySoundatLocation "/Game/Audio/Voice/Grand_Warrior_Cue.Grand_Warrior_Cue" _returnvalue "0, 0, 0" 1.0 1.0 0.0 0 0 0)))))
    (else
      (Pawn|Components|CharacterMovement|SetMovementMode (Variables|Character|GetCharacterMovement) "MOVE_None" 0))))

(event EventBeginPlay
  ;[1 1 1] Start/Stop Walking
  (Utilities|FlowControl|Sequence
    (:then_0
      (Utilities|FlowControl|Delay 3.0)
      (Utilities|FlowControl|DoOnce false
        (:Completed
          (Audio|PlaySoundatLocation "/Game/Audio/Voice/Practice_Cue.Practice_Cue" (Transformation|GetActorLocation) "0, 0, 0" 1.0 1.0 0.0 0 0 0))))
    (:then_1
      (bind _outactors (Actor|GetAllActorsOfClass "/Game/Blueprints/Assets/BP_Movepoint.BP_Movepoint_C")))))

(fn ConstructionScript)